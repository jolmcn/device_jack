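; Granular synth sound controller that plays motion SFX for a machine's main, base, arm, finger and laser movements.
; Movement events configure per-part synth components via macros and trigger notes, with main and base pitch following speed and reversal timelines.
; Drill hits run a timeline that sidechains main and base rotation volume.
; Test events map controller values onto arm synth parameters and print them for tuning defaults.
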(event `/Game/0_IO_Control/MIDI_Control/Inputs/BPI/BPI_UIControl.GrainPitchChange`
  (params (Vel :type "Float (single-precision)"))
  ;[1 0.05611 0] TESTING - Finding Best Defaults for Various SFX
  (bind _output_get (set `self.TestPitch` (`KismetMathLibrary.MapRangeClamped` Vel 0.0 1.0 0.9 1.1)))
  (`GranularSynth.SetGrainPitch` (`self.SFX_SC_ArmRotation`) _output_get (0.0 0.0))
  (`KismetSystemLibrary.PrintString` (`KismetStringLibrary.Conv_DoubleToString` _output_get) true true (struct :`G` 0.66 :`B` 1.0 :`A` 1.0) 10.0)
  (`GranularSynth.NoteOn` (`self.SFX_SC_ArmRotation`) 32.0 50 -1.0 :!label _label))

(event `/Game/0_IO_Control/MIDI_Control/Inputs/BPI/BPI_UIControl.AttackTimeChange`
  (params (Vel :type "Float (single-precision)"))
  ;[1 0.05611 0] TESTING - Finding Best Defaults for Various SFX
  (bind _output_get (set `self.TestAttackTime` (`KismetMathLibrary.MapRangeClamped` Vel 0.0 1.0 0.0 5.0)))
  (`GranularSynth.SetAttackTime` (`self.SFX_SC_ArmRotation`) _output_get)
  (`KismetSystemLibrary.PrintString` (`KismetStringLibrary.Conv_DoubleToString` _output_get) true true (struct :`G` 0.66 :`B` 1.0 :`A` 1.0) 10.0)
  (goto _label))

(event `/Game/0_IO_Control/MIDI_Control/Inputs/BPI/BPI_UIControl.DecayTimeChange`
  (params (Vel :type "Float (single-precision)"))
  ;[1 0.05611 0] TESTING - Finding Best Defaults for Various SFX
  (bind _output_get (set `self.TestDecayTime` (`KismetMathLibrary.MapRangeClamped` Vel 0.0 1.0 0.0 (`self.TestSoundwaveDuration`))))
  (`GranularSynth.SetDecayTime` (`self.SFX_SC_ArmRotation`) _output_get)
  (`KismetSystemLibrary.PrintString` (`KismetStringLibrary.Conv_DoubleToString` _output_get) true true (struct :`G` 0.66 :`B` 1.0 :`A` 1.0) 10.0)
  (goto _label))

(event `/Game/0_IO_Control/MIDI_Control/Inputs/BPI/BPI_UIControl.ReleaseTimeChange`
  (params (Vel :type "Float (single-precision)"))
  ;[1 0.05611 0] TESTING - Finding Best Defaults for Various SFX
  (bind _output_get (set `self.TestReleaseTime` (`KismetMathLibrary.MapRangeClamped` Vel 0.0 1.0 0.0 (`self.TestSoundwaveDuration`))))
  (`GranularSynth.SetReleaseTimeMsec` (`self.SFX_SC_ArmRotation`) _output_get)
  (`KismetSystemLibrary.PrintString` (`KismetStringLibrary.Conv_DoubleToString` _output_get) true true (struct :`G` 0.66 :`B` 1.0 :`A` 1.0) 10.0)
  (goto _label))

(event `/Game/0_IO_Control/MIDI_Control/Inputs/BPI/BPI_UIControl.GrainVolumeChange`
  (params (Vel :type "Float (single-precision)"))
  ;[1 0.05611 0] TESTING - Finding Best Defaults for Various SFX
  (bind _output_get (set `self.TestBaseVolume` (`KismetMathLibrary.MapRangeClamped` Vel 0.0 1.0 0.0 50.0)))
  (`GranularSynth.SetGrainVolume` (`self.SFX_SC_ArmRotation`) _output_get (0.0 0.0))
  (`KismetSystemLibrary.PrintString` (`KismetStringLibrary.Conv_DoubleToString` _output_get) true true (struct :`G` 0.66 :`B` 1.0 :`A` 1.0) 10.0)
  (goto _label))

(event `/Game/0_IO_Control/MIDI_Control/Inputs/BPI/BPI_UIControl.PlaybackSpeedChange`
  (params (Vel :type "Float (single-precision)"))
  ;[1 0.05611 0] TESTING - Finding Best Defaults for Various SFX
  (bind _output_get (set `self.TestPlayheadRate` (`KismetMathLibrary.MapRangeClamped` Vel 0.0 1.0 0.0 60.0)))
  (`GranularSynth.SetPlaybackSpeed` (`self.SFX_SC_ArmRotation`) _output_get)
  (`KismetSystemLibrary.PrintString` (`KismetStringLibrary.Conv_DoubleToString` _output_get) true true (struct :`G` 0.66 :`B` 1.0 :`A` 1.0) 10.0)
  (goto _label))

(event `/Game/0_IO_Control/MIDI_Control/Inputs/BPI/BPI_UIControl.SustainGainChange`
  (params (Vel :type "Float (single-precision)"))
  ;[1 0.05611 0] TESTING - Finding Best Defaults for Various SFX
  (bind _output_get (set `self.TestSustainGain` (`KismetMathLibrary.MapRangeClamped` Vel 0.0 1.0 0.0 5.0)))
  (`GranularSynth.SetSustainGain` (`self.SFX_SC_ArmRotation`) _output_get)
  (`KismetSystemLibrary.PrintString` (`KismetStringLibrary.Conv_DoubleToString` _output_get) true true (struct :`G` 0.66 :`B` 1.0 :`A` 1.0) 10.0)
  (goto _label))

(event `/Game/0_IO_Control/MIDI_Control/Inputs/BPI/BPI_UIControl.GrainDurationChange`
  (params (Vel :type "Float (single-precision)"))
  ;[1 0.05611 0] TESTING - Finding Best Defaults for Various SFX
  (bind _output_get (set `self.TestBaseDuration` (`KismetMathLibrary.MapRangeClamped` Vel 0.0 1.0 0.0 (`self.TestSoundwaveDuration`))))
  (`GranularSynth.SetGrainDuration` (`self.SFX_SC_ArmRotation`) _output_get (0.0 0.0))
  (`KismetSystemLibrary.PrintString` (`KismetStringLibrary.Conv_DoubleToString` _output_get) true true (struct :`G` 0.66 :`B` 1.0 :`A` 1.0) 10.0))

(event `/Game/0_IO_Control/MIDI_Control/Inputs/BPI/BPI_UIControl.GrainsPerSecondChange`
  (params (Vel :type "Float (single-precision)"))
  ;[1 0.05611 0] TESTING - Finding Best Defaults for Various SFX
  (bind _output_get (set `self.TestGrainsPerSecond` (`KismetMathLibrary.MapRangeClamped` Vel 0.0 1.0 1.0 20.0)))
  (`GranularSynth.SetGrainsPerSecond` (`self.SFX_SC_ArmRotation`) _output_get)
  (`KismetSystemLibrary.PrintString` (`KismetStringLibrary.Conv_DoubleToString` _output_get) true true (struct :`G` 0.66 :`B` 1.0 :`A` 1.0) 10.0)
  (goto _label))

(event `/Game/0_IO_Control/MIDI_Control/Inputs/BPI/BPI_UIControl.PlayheadLocationChange`
  (params (Vel :type "Float (single-precision)"))
  ;[1 0.05611 0] TESTING - Finding Best Defaults for Various SFX
  (bind _output_get (set `self.TestInPositionSecond` (`KismetMathLibrary.MapRangeClamped` Vel 0.0 1.0 0.0 (`self.TestSoundwaveDuration`))))
  (`GranularSynth.SetPlayheadTime` (`self.SFX_SC_ArmRotation`) _output_get 0.0 "FromBeginning")
  (`KismetSystemLibrary.PrintString` (`KismetStringLibrary.Conv_DoubleToString` _output_get) true true (struct :`G` 0.66 :`B` 1.0 :`A` 1.0) 10.0)
  (goto _label))

(event `self.ReceiveBeginPlay`
  ;[1 1 1] Setups
  (`|ExecutionSequence`
    (:`then_0`
      (`self.Set Defaults`)
      ;[1 0.928 0.4582] Keyboard Input
      (`self.EnableInput` (`GameplayStatics.GetPlayerController` 0)))
    (:`then_1`
      (`self.SC_SetDefaults` 0))
    (:`then_2`
      (set `self.Current_SC` null))))

(event `/Game/0_IO_Control/MIDI_Control/Inputs/BPI/BPI_nanoKONTROL.NK Cycle Button Press`
  ;[1 1 1] Switch Between Music/SFX Control
  (set `self.ControlSFX` (not (`self.ControlSFX`))))

(event `/Game/0_IO_Control/MIDI_Control/Inputs/BPI/BPI_SynthActivator.MainRotation`
  (params (Velocity :type "Float (single-precision)") (Clockwise :type Boolean))
  (bind _sfx_sc_mainrotation (`self.SFX_SC_MainRotation`))
  (bind _note (`self.Note`))
  ;[0.9922 0.4392 1] Synth SFX Control
  ;;[1 1 1] Main Rotation
  (if (== Velocity 0.0)
    (`GranularSynth.NoteOff` _sfx_sc_mainrotation _note false)
    (goto _label_2 :!via `Reset`)
    (else
      (`self.MACRO_SC_MainRotation` Velocity Clockwise)
      (`/Engine/EditorBlueprintResources/StandardMacros.DoOnce` false :!label _label_2
        (:`Completed`
          (`GranularSynth.NoteOn` _sfx_sc_mainrotation _note (`self.Velocity`) (`self.Duration`)))))))

(event `/Game/0_IO_Control/MIDI_Control/Inputs/BPI/BPI_SynthActivator.MainReversal`
  ;[0.9922 0.4392 1] Synth SFX Control
  ;;[1 1 1] Main Rotation
  (bind (_direction _pitchdown) (`Timeline|MainReverse` :!via `PlayFromStart`)
    (:`Update`
      (`GranularSynth.SetGrainPitch` (`self.SFX_SC_MainRotation`) (`KismetMathLibrary.MapRangeClamped` _pitchdown 1.0 0.0 (`self.MainRotationSpeed`)) (0.0 0.0)))))

(event `/Game/0_IO_Control/MIDI_Control/Inputs/BPI/BPI_SynthActivator.BaseRotation`
  (params (Velocity :type "Float (single-precision)"))
  (bind _sfx_sc_baserotation (`self.SFX_SC_BaseRotation`))
  (bind _note (`self.Note`))
  ;[0.9922 0.4392 1] Synth SFX Control
  ;;[1 1 1] Base Rotation
  (if (== Velocity 0.0)
    (`GranularSynth.NoteOff` _sfx_sc_baserotation _note true :!label _label_3)
    (goto _label_4 :!via `Reset`)
    (else
      (`self.MACRO_SC_BaseRotation` Velocity)
      (`/Engine/EditorBlueprintResources/StandardMacros.DoOnce` false :!label _label_4
        (:`Completed`
          (`GranularSynth.NoteOn` _sfx_sc_baserotation _note (`self.Velocity`) -1.0)
          (`KismetSystemLibrary.Delay` 0.2)
          (goto _label_4 :!via `Reset`))))))

(event `/Game/0_IO_Control/MIDI_Control/Inputs/BPI/BPI_SynthActivator.BaseOff`
  ;[0.9922 0.4392 1] Synth SFX Control
  ;;[1 1 1] Base Rotation
  (`KismetSystemLibrary.PrintString` "off")
  (goto _label_3))

(event `/Game/0_IO_Control/MIDI_Control/Inputs/BPI/BPI_SynthActivator.BaseReversal`
  ;[0.9922 0.4392 1] Synth SFX Control
  ;;[1 1 1] Base Rotation
  (bind (_direction _pitchdown) (`Timeline|BaseReverse` :!via `PlayFromStart`)
    (:`Update`
      (`GranularSynth.SetGrainPitch` (`self.SFX_SC_BaseRotation`) (`KismetMathLibrary.MapRangeClamped` _pitchdown 1.0 0.0 (`self.BaseRotationSpeed`)) (0.0 0.0)))))

(event `/Game/0_IO_Control/MIDI_Control/Inputs/BPI/BPI_SynthActivator.ArmRotation`
  (params (Velocity :type "Float (single-precision)"))
  ;[0.9922 0.4392 1] Synth SFX Control
  ;;[1 1 1] Arm Rotation
  (`self.MACRO_SC_ArmRotation` Velocity)
  (`/Engine/EditorBlueprintResources/StandardMacros.DoOnce` false :!label _label_5
    (:`Completed`
      (`GranularSynth.NoteOn` (`self.SFX_SC_ArmRotation`) (`self.Note`) (`self.Velocity`) 0.3)
      (`KismetSystemLibrary.Delay` 0.2)
      (goto _label_5 :!via `Reset`))))

(event `/Game/0_IO_Control/MIDI_Control/Inputs/BPI/BPI_SynthActivator.FingerRotation`
  (params (Velocity :type "Float (single-precision)"))
  ;[0.9922 0.4392 1] Synth SFX Control
  ;;[1 1 1] Finger Rotation
  (`self.MACRO_SC_FingerRotation` Velocity)
  (`/Engine/EditorBlueprintResources/StandardMacros.DoOnce` false :!label _label_6
    (:`Completed`
      (`GranularSynth.NoteOn` (`self.SFX_SC_FingerRotation`) (`self.Note`) (`self.Velocity`) 0.3)
      (`KismetSystemLibrary.Delay` 0.3)
      (goto _label_6 :!via `Reset`))))

(event `/Game/0_IO_Control/MIDI_Control/Inputs/BPI/BPI_SynthActivator.FingerLocation`
  (params (Velocity :type "Float (single-precision)"))
  ;[0.9922 0.4392 1] Synth SFX Control
  ;;[1 1 1] Finger Location
  (`self.MACRO_SC_FingerLocation` Velocity)
  (`/Engine/EditorBlueprintResources/StandardMacros.DoOnce` false :!label _label_7
    (:`Completed`
      (`GranularSynth.NoteOn` (`self.SFX_SC_FingerLocation`) (`self.Note`) (`self.Velocity`) 0.25)
      (`KismetSystemLibrary.Delay` 0.25)
      (goto _label_7 :!via `Reset`))))

(event `/Game/0_IO_Control/MIDI_Control/Inputs/BPI/BPI_SynthActivator.LaserRotation`
  (params (Velocity :type "Float (single-precision)"))
  (bind _sfx_sc_laserrotation (`self.SFX_SC_LaserRotation`))
  (bind _note (`self.Note`))
  ;[0.9922 0.4392 1] Synth SFX Control
  ;;[1 1 1] Laser Rotation
  (`self.MACRO_SC_LaserRotation` Velocity)
  (`GranularSynth.NoteOn` _sfx_sc_laserrotation _note (`self.Velocity`) (`self.Duration`))
  (`KismetSystemLibrary.Delay` 0.2)
  (`GranularSynth.NoteOff` _sfx_sc_laserrotation _note false))

(event `/Game/0_IO_Control/MIDI_Control/Inputs/BPI/BPI_SynthActivator.Drills`
  (params (Velocity :type "Float (single-precision)"))
  ;[0.9922 0.4392 1] Synth SFX Control
  ;;[1 1 1] Drill Hit
  (bind _output_get (set `self.SidechainValue` Velocity))
  (bind (_direction _alpha) (`Timeline|Timeline_0` :!via `PlayFromStart`)
    (:`Update`
      (`self.SideChains` (`KismetMathLibrary.Lerp` 0.0 _output_get _alpha) _output_get))))

(fn `UserConstructionScript`)